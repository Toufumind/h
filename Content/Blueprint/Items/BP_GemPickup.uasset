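; A gem pickup actor that gives its configured gem type to a SpriteAssembleCharacter that overlaps its box.
; If AddGem succeeds, it refreshes the WBP_GemHUD found in the viewport and destroys itself.
; Otherwise it starts that HUD's swap mode, passing the new gem type and itself as the actor to destroy.
; The construction script tints the Paper sprite by gem type: split projectile, damage up or lifesteal.
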(event OnComponentBeginOverlap(Box)
  (params (OverlappedComponent :type Primitive%20Component%20Object%20Reference) (OtherActor :type Actor%20Object%20Reference) (OtherComp :type Primitive%20Component%20Object%20Reference) (OtherBodyIndex :type Integer) (bFromSweep :type Boolean) (SweepResult :type Hit%20Result%20Structure%20%28by%20ref%29))
  (bind _assprite_assemble_character (Utilities|Casting|CastToSpriteAssembleCharacter OtherActor))
  (bind _returnvalue (Class|SpriteAssembleCharacter|AddGem _assprite_assemble_character (Variables|Default|GetGemTypeToGive)))
  (if _returnvalue
    (bind _foundwidgets (Widget|GetAllWidgetsOfClass "/Game/GUI/WBP_GemHUD.WBP_GemHUD_C" true))
    (Default|UpdateGemUI (Utilities|Array|Get(acopy) _foundwidgets))
    (Actor|DestroyActor)
    (else
      (bind _foundwidgets_2 (Widget|GetAllWidgetsOfClass "/Game/GUI/WBP_GemHUD.WBP_GemHUD_C" true))
      (Default|StartSwapMode (Utilities|Array|Get(acopy) _foundwidgets_2) (Variables|Default|GetGemTypeToGive) self))))

(fn ConstructionScript
  (bind _papersprite (Variables|Default|GetPaperSprite))
  (switch Utilities|FlowControl|Switch|SwitchonEGemType (Variables|Default|GetGemTypeToGive)
    (:Split
      (Sprite|SetSpriteColor _papersprite "(R=255.000000,G=0.000000,B=0.000000,A=1.000000)"))
    (:DamageUp
      (Sprite|SetSpriteColor _papersprite "(R=0.000000,G=255.000000,B=0.000000,A=1.000000)"))
    (:Lifesteal
      (Sprite|SetSpriteColor _papersprite "(R=0.000000,G=0.000000,B=255.000000,A=1.000000)"))))